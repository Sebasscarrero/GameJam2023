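; BP_PlayerSoulCounter, filed under Components, keeps a running tally of good versus bad souls for the player.
; SoulCounter resets to zero on BeginPlay, and the UpdateSoulCounter event raises it by one for a good soul or lowers it otherwise.
; The float is truncated to an integer for each step and converted back, with no clamping or change notification.
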(event `self.ReceiveBeginPlay`
  (set `self.SoulCounter` 0.0))

(event `UpdateSoulCounter`
  (params (`IsGoodSoul?` :type Boolean))
  (if `IsGoodSoul?`
    (bind _result (`/Engine/EditorBlueprintResources/StandardMacros.IncrementInt` (`KismetMathLibrary.FTrunc` (`self.SoulCounter`)))
      (:`  `
        (set `self.SoulCounter` (`KismetMathLibrary.Conv_IntToDouble` _result))))
    (else
      (bind _result_2 (`/Engine/EditorBlueprintResources/StandardMacros.DecrementInt` (`KismetMathLibrary.FTrunc` (`self.SoulCounter`)))
        (:`  `
          (set `self.SoulCounter` (`KismetMathLibrary.Conv_IntToDouble` _result_2)))))))