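; Trigger actor that teleports any BP_Enemy overlapping ActivateTrigger to PointToTeleport with a morph effect.
; It spawns a BP_Clone at the enemy's old transform, zeroes the MPC_Morph Amount1 parameter, then moves the enemy.
; InitializeEffect feeds the clone and enemy skeletal meshes to Niagara as morph endpoints.
; Two timelines, started together, drive Amount1 and Amount2 in the parameter collection to animate the transition.
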(event `self.ActivateTrigger.OnComponentBeginOverlap`
  (params (OverlappedComponent :type "PrimitiveComponent Object Reference") (OtherActor :type "Actor Object Reference") (OtherComp :type "PrimitiveComponent Object Reference") (OtherBodyIndex :type Integer) (bFromSweep :type Boolean) (SweepResult :type "HitResult Structure (by ref)"))
  (bind _secondactor (`self.SecondActor`))
  (bind _asbp_enemy (cast `/Game/GameJam2023/Character/Enemy/BP_Enemy` OtherActor))
  (set `self.SecondActor` _asbp_enemy)
  (bind _returnvalue (`|SpawnActorFromClass` "/Game/GameJam2023/Character/Enemy/BP_Clone.BP_Clone_C" (`self.GetTransform` _asbp_enemy) "AlwaysSpawn" "OverrideRootScale" null null))
  (set `self.FirstActor` _returnvalue)
  (bind _returnvalue_2 (`KismetMaterialLibrary.GetScalarParameterValue` "/Game/GameJam2023/Character/Enemy/MPC_Morph.MPC_Morph" "Amount1"))
  (set `self.DefaultValue` _returnvalue_2)
  (`KismetMaterialLibrary.SetScalarParameterValue` "/Game/GameJam2023/Character/Enemy/MPC_Morph.MPC_Morph" "Amount1")
  (`self.K2_TeleportTo` _secondactor (`SceneComponent.K2_GetComponentLocation` (`self.PointToTeleport`)) (`self.K2_GetActorRotation` _secondactor))
  (`self.InitializeEffect`))

(event `InitializeEffect`
  (`NiagaraFunctionLibrary.OverrideSystemUserVariableSkeletalMeshComponent` (`self.Niagara`) "SkeletalMeshA" (`self.GetComponentByClass` (`self.FirstActor`) "/Script/Engine.SkeletalMeshComponent"))
  (`NiagaraFunctionLibrary.OverrideSystemUserVariableSkeletalMeshComponent` null "SkeletalMeshB" (`self.GetComponentByClass` (`self.SecondActor`) "/Script/Engine.SkeletalMeshComponent"))
  (`|ExecutionSequence`
    (:`then_0`
      (bind (_direction _newtrack_0) (`Timeline|Timeline` :!via `PlayFromStart`)
        (:`Update`
          (`KismetMaterialLibrary.SetScalarParameterValue` "/Game/GameJam2023/Character/Enemy/MPC_Morph.MPC_Morph" "Amount1" _newtrack_0))))
    (:`then_1`
      (bind (_direction_2 _newtrack_0_2) (`Timeline|Timeline_0` :!via `PlayFromStart`)
        (:`Update`
          (`KismetMaterialLibrary.SetScalarParameterValue` "/Game/GameJam2023/Character/Enemy/MPC_Morph.MPC_Morph" "Amount2" _newtrack_0_2))))))

(fn `UserConstructionScript`)