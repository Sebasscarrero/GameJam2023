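; Destructible prop that shatters when punched by the player and spawns a BP_Soul.
; A Capsule overlap with a component whose last tag is "Punch" applies massive impulse damage from the punch location and disables collision.
; A DoOnce gates the soul spawn, placed at the capsule's XY just below player height.
; Timeline-based sink-and-destroy despawn is disconnected, leaving Tick printing its debug position.
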(event OnComponentBeginOverlap(Capsule)
  (params (OverlappedComponent :type Primitive%20Component%20Object%20Reference) (OtherActor :type Actor%20Object%20Reference) (OtherComp :type Primitive%20Component%20Object%20Reference) (OtherBodyIndex :type Integer) (bFromSweep :type Boolean) (SweepResult :type Hit%20Result%20Structure%20%28by%20ref%29))
  (bind _destructible (Variables|Default|GetDestructible))
  (Variables|Default|SetPlayer (.AsThird%20Person%20Character (Utilities|Casting|CastToThirdPersonCharacter (Game|Player|GetPlayerPawn 0))))
  (for _array_element (Variables|/Script/Engine.ActorComponent|GetComponentTags OtherComp)
    (Variables|Default|SetbIsPunch (Utilities|Name|Equal(Name) _array_element "Punch")))
  (if (Variables|Default|GetbIsPunch)
    (Components|Activation|Activate (Variables|Default|GetDestructible) false)
    (Physics|SetSimulatePhysics _destructible true)
    (Class|DestructibleComponent|ApplyDamage _destructible 1e+06 (Transformation|GetWorldLocation (Variables|/Game/ThirdPersonBP/Blueprints/ThirdPersonCharacter.ThirdPersonCharacter_C|GetPunchCollision (Variables|Default|GetPlayer))) (Transformation|GetActorForwardVector (Variables|Default|GetPlayer)) 1e+03)
    (CallFunction|SpawnSoul)
    (Collision|SetCollisionEnabled (Variables|Default|GetCapsule) "NoCollision")))

(event Custom|SpawnSoul
  (bind _capsule (Variables|Default|GetCapsule))
  (bind _returnvalue (Transformation|GetWorldLocation _capsule))
  (Utilities|FlowControl|DoOnce false
    (:Completed
      (Game|SpawnActorfromClass "/Game/GameJam2023/Blueprints/General/Soul/BP_Soul.BP_Soul_C" (Math|Transform|MakeTransform (Math|Vector|MakeVector (.x _returnvalue) (.y _returnvalue) (- (.z (Transformation|GetActorLocation (Variables|Default|GetPlayer))) 5e+01)) "0, 0, 0" "0.600000,0.600000,0.600000") "Undefined" 0 false 0 false 0))))

(event EventTick
  (params (DeltaSeconds :type Float%20%28single-precision%29))
  (bind _destructible (Variables|Default|GetDestructible))
  (bind _returnvalue (Transformation|GetWorldLocation _destructible))
  (Development|PrintString (Utilities|String|ToString(Vector) (Math|Vector|Lerp(Vector) (Transformation|GetWorldLocation _destructible) (Math|Vector|MakeVector (.x _returnvalue) (.y _returnvalue) -1e+05) (stale _speed))) true true "(R=1.000000,G=0.000000,B=0.005787,A=1.000000)" 0.001))

(event EventBeginPlay
  (Class|DestructibleComponent|SetDestructibleMesh (Variables|Default|GetDestructible) (Variables|Default|GetDestructibleObject)))

(fn ConstructionScript)