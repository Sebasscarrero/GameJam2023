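; BP_Casillero is an actor that gives its static mesh a random look when play begins.
; On BeginPlay it picks an index into its Materials array and applies that material to slot 0, falling back to the first entry when the validity check fails.
; The random range includes the array length, and the pure random node can roll again after the check, so the applied index may differ from the validated one.
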(event `self.ReceiveBeginPlay`
  (bind _materials (`self.Materials`))
  (bind _returnvalue (`KismetMathLibrary.RandomIntegerInRange` 0 (`KismetArrayLibrary.Array_Length` (`self.Materials`))))
  (if (`KismetArrayLibrary.Array_IsValidIndex` _materials _returnvalue)
    (`PrimitiveComponent.SetMaterial` (`self.StaticMesh`) 0 (`|GetArrayItem` _materials _returnvalue))
    (else
      (`PrimitiveComponent.SetMaterial` (`self.StaticMesh`) 0 (`|GetArrayItem` (`self.Materials`))))))

(fn `UserConstructionScript`)