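; BP_TearingEye is a Phase 4 game jam actor that continuously wanders to random points on its horizontal plane from BeginPlay.
; Each cycle picks an XY goal within fixed world bounds, keeps the current Z, and restarts the MoveActor timeline at a random play rate.
; The timeline lerps from the current location toward the goal with collision sweep, then repeats after a short delay.
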(event `self.ReceiveBeginPlay`
  (`self.MoveToRandomLocation`))

(event `MoveToRandomLocation`
  (bind (_returnvalue_x _returnvalue_y _returnvalue_z) (`KismetMathLibrary.BreakVector` (`self.K2_GetActorLocation`)))
  (set `self.GoalLocation` (`KismetMathLibrary.MakeVector` (`KismetMathLibrary.RandomFloatInRange` 1000.0 -1000.0) (`KismetMathLibrary.RandomFloatInRange` 750.0 -750.0) _returnvalue_z))
  (`TimelineComponent.SetPlayRate` (`self.MoveActor`) (`KismetMathLibrary.RandomFloatInRange` 10.0 20.0))
  (bind (_direction _speedmove) (`Timeline|MoveActor` :!via `PlayFromStart`)
    (:`Update`
      (`self.K2_SetActorLocation` (`KismetMathLibrary.VLerp` (`self.K2_GetActorLocation`) (`self.GoalLocation`) _speedmove) true))
    (:`Finished`
      (`KismetSystemLibrary.Delay` 0.2)
      (`self.MoveToRandomLocation`))))

(fn `UserConstructionScript`)