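; BP_Soul_Child is a short-lived child actor from the Phase 4 game jam content that adds a debug trace to its parent's behavior.
; On BeginPlay it runs the parent logic, then line traces for WorldStatic objects along the static mesh's negative up vector, drawing the line.
; The trace result is unused, and the actor destroys itself after a brief delay.
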(event `self.ReceiveBeginPlay`
  (bind _returnvalue (`self.K2_GetActorLocation`))
  (`parent.ReceiveBeginPlay`)
  (`KismetSystemLibrary.LineTraceSingleForObjects` :`Start` _returnvalue :`End` (+ _returnvalue (* (`SceneComponent.GetUpVector` (`self.StaticMesh`)) -1500.0)) :`ObjectTypes` (`|MakeArray` "ObjectTypeQuery1" :!type "EObjectTypeQuery Enum") :`DrawDebugType` "ForDuration" :`DrawTime` 2.0)
  (`KismetSystemLibrary.Delay` 2.0)
  (`self.K2_DestroyActor`))

(fn `UserConstructionScript`
  (`parent.UserConstructionScript`))