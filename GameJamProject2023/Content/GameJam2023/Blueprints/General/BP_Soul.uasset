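; BP_Soul is a soul pickup that randomly becomes good or bad on BeginPlay, setting its material color and homing timeline play rate, much slower for bad souls.
; While the ThirdPersonCharacter is inside MoveToPlayerCollision, the timeline lerps the soul horizontally toward them, keeping its height.
; Overlapping the Sphere passes the soul type to the character's PlayerSoulCounter, spawns an explosion effect and destroys the soul.
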(event `self.ReceiveBeginPlay`
  (set `self.bIsGoodSoul?` (`KismetMathLibrary.RandomBool`))
  (bind _returnvalue (`PrimitiveComponent.CreateDynamicMaterialInstance` (`self.StaticMesh`) 0 "/Game/GameJam2023/Blueprints/General/M_Soul.M_Soul" "None"))
  (if (`self.bIsGoodSoul?`)
    (`MaterialInstanceDynamic.SetVectorParameterValue` _returnvalue "SoulColor" (struct :`G` 0.971556 :`B` 1.0 :`A` 1.0))
    (`TimelineComponent.SetPlayRate` (`self.MoveSoulToPlayer`) 1.0)
    (else
      (`MaterialInstanceDynamic.SetVectorParameterValue` _returnvalue "SoulColor" (struct :`R` 0.413602 :`B` 0.595833 :`A` 1.0))
      (`TimelineComponent.SetPlayRate` (`self.MoveSoulToPlayer`) 0.15))))

(event `self.Sphere.OnComponentBeginOverlap`
  (params (OverlappedComponent :type "PrimitiveComponent Object Reference") (OtherActor :type "Actor Object Reference") (OtherComp :type "PrimitiveComponent Object Reference") (OtherBodyIndex :type Integer) (bFromSweep :type Boolean) (SweepResult :type "HitResult Structure (by ref)"))
  (bind _asthird_person_character (cast `/Game/ThirdPersonBP/Blueprints/ThirdPersonCharacter` OtherActor))
  (bind _returnvalue (`self.GetComponentByClass` _asthird_person_character "/Game/GameJam2023/Components/PlayerSoulCounter.PlayerSoulCounter_C"))
  (`/Engine/EditorBlueprintResources/StandardMacros.IsValid` _returnvalue
    (:`Is Valid`
      (`/Game/GameJam2023/Components/PlayerSoulCounter.UpdateSoulCounter` _returnvalue (`self.bIsGoodSoul?`))
      (`GameplayStatics.SpawnEmitterAtLocation` "/Game/StarterContent/Particles/P_Explosion.P_Explosion" (`self.K2_GetActorLocation`))
      (`self.K2_DestroyActor`))))

(event `self.MoveToPlayerCollision.OnComponentBeginOverlap`
  (params (OverlappedComponent :type "PrimitiveComponent Object Reference") (OtherActor :type "Actor Object Reference") (OtherComp :type "PrimitiveComponent Object Reference") (OtherBodyIndex :type Integer) (bFromSweep :type Boolean) (SweepResult :type "HitResult Structure (by ref)"))
  (bind (_returnvalue_x _returnvalue_y _returnvalue_z) (`KismetMathLibrary.BreakVector` (`self.K2_GetActorLocation`)))
  (bind _asthird_person_character (cast `/Game/ThirdPersonBP/Blueprints/ThirdPersonCharacter` OtherActor))
  (bind (_direction _speed) (`Timeline|MoveSoulToPlayer` :!via `PlayFromStart` :!label _label)
    (:`Update`
      (`/Engine/EditorBlueprintResources/StandardMacros.IsValid` _asthird_person_character
        (:`Is Valid`
          (bind (_returnvalue_x_2 _returnvalue_y_2) (`KismetMathLibrary.BreakVector` (`self.K2_GetActorLocation` _asthird_person_character)))
          (`self.K2_SetActorLocation` (`KismetMathLibrary.VLerp` (`KismetMathLibrary.MakeVector` _returnvalue_x _returnvalue_y _returnvalue_z) (`KismetMathLibrary.MakeVector` _returnvalue_x_2 _returnvalue_y_2 _returnvalue_z) _speed)))))))

(event `self.MoveToPlayerCollision.OnComponentEndOverlap`
  (params (OverlappedComponent :type "PrimitiveComponent Object Reference") (OtherActor :type "Actor Object Reference") (OtherComp :type "PrimitiveComponent Object Reference") (OtherBodyIndex :type Integer))
  (cast `/Game/ThirdPersonBP/Blueprints/ThirdPersonCharacter` OtherActor)
  (goto _label :!via `Stop`))

(fn `UserConstructionScript`)