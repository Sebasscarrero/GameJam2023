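; Collectible soul that bobs and randomly becomes good or bad, setting its color, Niagara tint and homing speed, and registers with GM_GameMode.
; Entering the outer collision starts a timeline that pulls it horizontally toward the player, much slower for bad souls.
; Touching the inner sphere updates BP_PlayerSoulCounter, spawns an explosion and destroys it.
; IsFinalFloatingMode skips that setup, deactivates both collisions and moves it along a spline.
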(event `SetSoulFloatingMovement`
  (bind _soulfloatingspline (`self.SoulFloatingSpline`))
  (`ActorComponent.Deactivate` (`self.MoveToPlayerCollision`))
  (`ActorComponent.Deactivate` (`self.Sphere`))
  (bind (_direction _speed) (`Timeline|SoulFloatingMovement`)
    (:`Update`
      (`self.K2_SetActorTransform` (`KismetMathLibrary.MakeTransform` (`SplineComponent.GetLocationAtDistanceAlongSpline` _soulfloatingspline (`KismetMathLibrary.Lerp` 0.0 (`SplineComponent.GetSplineLength` (`self.SoulFloatingSpline`)) _speed) "World") (`SplineComponent.GetRotationAtDistanceAlongSpline` _soulfloatingspline 0.0 "Local"))))))

(event `self.ReceiveBeginPlay`
  (bind _valuenotgood (`self.ValueNotGood`))
  (bind _valuegood (`self.ValueGood`))
  (`self.BobbingUp`)
  (if (`self.bIsFinalFloatingMode`)
    (`self.SetSoulFloatingMovement`)
    (else
      (`|ExecutionSequence`
        (:`then_0`
          (set `self.bIsGoodSoul?` (`KismetMathLibrary.RandomBool`)))
        (:`then_1`
          (bind _asgm_game_mode (cast `/Game/GameJam2023/Blueprints/General/GM_GameMode` (`GameplayStatics.GetGameMode`)))
          (`/Game/GameJam2023/Blueprints/General/GM_GameMode.AddSoulToTotalSpawned` _asgm_game_mode))
        (:`then_2`
          (bind _returnvalue (`PrimitiveComponent.CreateDynamicMaterialInstance` (`self.StaticMesh`) 0 "/Game/GameJam2023/Blueprints/General/Soul/M_Soul.M_Soul" "None"))
          (if (`self.bIsGoodSoul?`)
            (`MaterialInstanceDynamic.SetVectorParameterValue` _returnvalue "SoulColor" _valuegood)
            (`NiagaraComponent.SetNiagaraVariableLinearColor` (`self.Niagara`) "LinearColor" _valuegood)
            (`TimelineComponent.SetPlayRate` (`self.MoveSoulToPlayer`) 1.0)
            (else
              (`MaterialInstanceDynamic.SetVectorParameterValue` _returnvalue "SoulColor" _valuenotgood)
              (`NiagaraComponent.SetNiagaraVariableLinearColor` (`self.Niagara`) "LinearColor" _valuenotgood)
              (`TimelineComponent.SetPlayRate` (`self.MoveSoulToPlayer`) 0.15))))))))

(event `BobbingUp`
  (bind (_direction _bobbingup) (`Timeline|Movement`)
    (:`Update`
      (`SceneComponent.K2_AddLocalOffset` (`self.StaticMesh`) _bobbingup false false))))

(event `self.Sphere.OnComponentBeginOverlap`
  (params (OverlappedComponent :type "PrimitiveComponent Object Reference") (OtherActor :type "Actor Object Reference") (OtherComp :type "PrimitiveComponent Object Reference") (OtherBodyIndex :type Integer) (bFromSweep :type Boolean) (SweepResult :type "HitResult Structure (by ref)"))
  (bind _asthird_person_character (cast `/Game/ThirdPersonBP/Blueprints/ThirdPersonCharacter` OtherActor))
  (bind _returnvalue (`self.GetComponentByClass` _asthird_person_character "/Game/GameJam2023/Components/BP_PlayerSoulCounter.BP_PlayerSoulCounter_C"))
  (`/Engine/EditorBlueprintResources/StandardMacros.IsValid` _returnvalue
    (:`Is Valid`
      (`/Game/GameJam2023/Components/BP_PlayerSoulCounter.UpdateSoulCounter` _returnvalue (`self.bIsGoodSoul?`))
      (`GameplayStatics.SpawnEmitterAtLocation` "/Game/StarterContent/Particles/P_Explosion.P_Explosion" (`self.K2_GetActorLocation`))
      (`self.K2_DestroyActor`))))

(event `self.MoveToPlayerCollision.OnComponentBeginOverlap`
  (params (OverlappedComponent :type "PrimitiveComponent Object Reference") (OtherActor :type "Actor Object Reference") (OtherComp :type "PrimitiveComponent Object Reference") (OtherBodyIndex :type Integer) (bFromSweep :type Boolean) (SweepResult :type "HitResult Structure (by ref)"))
  (bind (_returnvalue_x _returnvalue_y _returnvalue_z) (`KismetMathLibrary.BreakVector` (`self.K2_GetActorLocation`)))
  (bind _asthird_person_character (cast `/Game/ThirdPersonBP/Blueprints/ThirdPersonCharacter` OtherActor))
  (bind (_direction _speed) (`Timeline|MoveSoulToPlayer` :!via `PlayFromStart`)
    (:`Update`
      (`/Engine/EditorBlueprintResources/StandardMacros.IsValid` _asthird_person_character
        (:`Is Valid`
          (bind (_returnvalue_x_2 _returnvalue_y_2) (`KismetMathLibrary.BreakVector` (`self.K2_GetActorLocation` _asthird_person_character)))
          (`self.K2_SetActorLocation` (`KismetMathLibrary.VLerp` (`KismetMathLibrary.MakeVector` _returnvalue_x _returnvalue_y _returnvalue_z) (`KismetMathLibrary.MakeVector` _returnvalue_x_2 _returnvalue_y_2 _returnvalue_z) _speed)))))))

(event `self.MoveToPlayerCollision.OnComponentEndOverlap`
  (params (OverlappedComponent :type "PrimitiveComponent Object Reference") (OtherActor :type "Actor Object Reference") (OtherComp :type "PrimitiveComponent Object Reference") (OtherBodyIndex :type Integer)))

(fn `UserConstructionScript`)