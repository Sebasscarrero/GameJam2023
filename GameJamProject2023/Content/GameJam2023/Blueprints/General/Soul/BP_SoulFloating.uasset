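; BP_SoulFloating spawns souls in final floating mode along its spline, apparently to visualise the final score.
; A looping timer spawns one BP_Soul at a time while the Test counter lasts, passing it the spline and storing it in Souls.
; Each soul is flagged good or bad by comparing the countdown against the GameMode's FinalScorePercentage divided by ten.
; Tick prints the soul count as debug text.
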(event `self.ReceiveBeginPlay`
  (`KismetSystemLibrary.K2_SetTimerDelegate` (delegate `SpawnSoul`) 0.5 true)
  (bind _asgm_game_mode (cast `/Game/GameJam2023/Blueprints/General/GM_GameMode` (`GameplayStatics.GetGameMode`)))
  (set `self.GM` _asgm_game_mode))

(event `SpawnSoul`
  (if (> (`self.Test`) 0.0)
    (bind _returnvalue (`|SpawnActorFromClass` "/Game/GameJam2023/Blueprints/General/Soul/BP_Soul.BP_Soul_C" (`SceneComponent.GetRelativeTransform` (`self.SoulFloatingSpline`)) "Undefined" "OverrideRootScale" null true (`self.SoulFloatingSpline`) (>= (`self.Test`) (/ (`/Game/GameJam2023/Blueprints/General/GM_GameMode.FinalScorePercentage` (`self.GM`)) 10.0)) null)) ; Set Final Floating Mode TRUE
    (`KismetArrayLibrary.Array_Add` (`self.Souls`) _returnvalue)
    (set `self.Test` (- (`self.Test`) 1.0))))

(event `self.ReceiveTick`
  (params (DeltaSeconds :type "Float (single-precision)"))
  (`KismetSystemLibrary.PrintString` (`KismetStringLibrary.Concat_StrStr` "Append: " (`KismetStringLibrary.Conv_IntToString` (`KismetArrayLibrary.Array_Length` (`self.Souls`))) " - ") true false (struct :`R` 1.0 :`G` 0.067256 :`A` 1.0) 0.001))

(fn `UserConstructionScript`)