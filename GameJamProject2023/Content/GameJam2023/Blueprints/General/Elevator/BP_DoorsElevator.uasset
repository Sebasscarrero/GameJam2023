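; Elevator door actor with two panels that the player slides open and closed with the Interactuar input.
; Entering the trigger box enables input and shows a prompt; a FlipFlop plays or reverses a timeline that offsets the panels in opposite directions.
; Leaving clears the camera timer handle and, if the doors are fully open, disables input and closes them.
; Camera shake events remain, but the nodes that start their looping timers are disconnected.
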(event `self.ReceiveBeginPlay`
  (set `self.MoveDoor1` (`SceneComponent.RelativeLocation` (`self.Door1`)))
  (set `self.MoveDoor2` (`SceneComponent.RelativeLocation` (`self.Door2`))))

(event `InputAction|Interactuar`
  (params (Key :type "Key Structure"))
  (:`Pressed`
    (`TimelineComponent.SetPlayRate` (`self.Door`) 5.0)
    (`/Engine/EditorBlueprintResources/StandardMacros.FlipFlop`
      (:`A`
        (bind (_direction _newtrack_0) (`Timeline|Door` :!label _label)
          (:`Update`
            (`SceneComponent.K2_SetRelativeLocation` (`self.Door1`) (+ (`self.MoveDoor1`) (`KismetMathLibrary.MakeVector` _newtrack_0)) false false)
            (`SceneComponent.K2_SetRelativeLocation` (`self.Door2`) (- (`self.MoveDoor2`) (`KismetMathLibrary.MakeVector` _newtrack_0)) false false))))
      (:`B`
        (goto _label :!via `Reverse`)))))

(event `self.Box.OnComponentEndOverlap`
  (params (OverlappedComponent :type "PrimitiveComponent Object Reference") (OtherActor :type "Actor Object Reference") (OtherComp :type "PrimitiveComponent Object Reference") (OtherBodyIndex :type Integer))
  (bind _door (`self.Door`))
  (cast `/Game/ThirdPersonBP/Blueprints/ThirdPersonCharacter` OtherActor)
  (bind _output_get (set `self.StopCamera` (struct)))
  (`KismetSystemLibrary.K2_ClearAndInvalidateTimerHandle` _output_get)
  (if (== (`TimelineComponent.GetPlaybackPosition` _door) (`TimelineComponent.GetTimelineLength` _door))
    (`self.DisableInput` (`GameplayStatics.GetPlayerController` 0))
    (goto _label :!via `Reverse`)))

(event `self.Box.OnComponentBeginOverlap`
  (params (OverlappedComponent :type "PrimitiveComponent Object Reference") (OtherActor :type "Actor Object Reference") (OtherComp :type "PrimitiveComponent Object Reference") (OtherBodyIndex :type Integer) (bFromSweep :type Boolean) (SweepResult :type "HitResult Structure (by ref)"))
  (cast `/Game/ThirdPersonBP/Blueprints/ThirdPersonCharacter` OtherActor)
  (`self.EnableInput` (`GameplayStatics.GetPlayerController` 0))
  (`KismetSystemLibrary.PrintString` "Press H to Open" true false (struct :`G` 0.66 :`B` 1.0 :`A` 1.0) 1.0))

(event `MovementCamera`
  (set `self.CameraShake1` (`self.CameraShake1`))
  (bind _returnvalue (`PlayerCameraManager.StartCameraShake` :`self` (`GameplayStatics.GetPlayerCameraManager` 0) :`ShakeClass` "/Game/GameJam2023/Blueprints/CameraShake/CameraShake.CameraShake_C"))
  (set `self.CameraMove` _returnvalue))

(event `s`
  (if (`self.CameraShake`)
    (`GameplayStatics.PlayWorldCameraShake` "/Script/GameplayCameras.MatineeCameraShake" (`self.K2_GetActorLocation`) 0.0 500.0)
    (else
      (`KismetSystemLibrary.K2_ClearAndInvalidateTimerHandle` (`self.NewVar_0`)))))

(fn `UserConstructionScript`)