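; Game jam game mode that caches the third-person player and tallies soul collection.
; SetFinalSoulScore reads the player's soul counter, prints a percentage computed from hard-coded placeholder inputs, then spawns a BP_SoulFloating attached above the player with the caught count.
; AddSoulToTotalSpawned increments the spawned total used in that printout.
; VerificaQuest only prints a debug message for the Villano objective, and the Testing timer is disconnected.
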(event `self.ReceiveBeginPlay`
  (bind _asthird_person_character (cast `/Game/ThirdPersonBP/Blueprints/ThirdPersonCharacter` (`GameplayStatics.GetPlayerPawn` 0)))
  (set `self.Player` _asthird_person_character))

(event `Testing`
  (`self.SetFinalSoulScore`))

(event `SetFinalSoulScore`
  (bind _player (`self.Player`))
  (bind _returnvalue (`self.GetComponentByClass` _player "/Game/GameJam2023/Components/BP_PlayerSoulCounter.BP_PlayerSoulCounter_C"))
  (`/Engine/EditorBlueprintResources/StandardMacros.IsValid` _player
    (:`Is Valid`
      (`/Engine/EditorBlueprintResources/StandardMacros.IsValid` _returnvalue
        (:`Is Valid`
          (set `self.CaughtSouls` (`/Game/GameJam2023/Components/BP_PlayerSoulCounter.SoulCounter` _returnvalue))
          (bind _finalpercentaje (`self.Set Percentage Score` 6.0 10.0))
          (set `self.FinalScorePercentage` _finalpercentaje)
          (`KismetSystemLibrary.PrintString` (`KismetStringLibrary.Concat_StrStr` "Caught Souls: " (`KismetStringLibrary.Conv_IntToString` (`KismetMathLibrary.Round` (`self.CaughtSouls`))) " / Total Souls: " (`KismetStringLibrary.Conv_IntToString` (`KismetMathLibrary.Round` (`self.TotalSoulsSpawned`))) " - FINAL PERCENTAGE: " (`KismetStringLibrary.Conv_DoubleToString` _finalpercentaje) "%") true false (struct :`R` 0.851326 :`B` 1.0 :`A` 1.0) 15.0)
          (`self.CreateSoulFloatingSpline`))))))

(event `AddSoulToTotalSpawned`
  (bind _result (`/Engine/EditorBlueprintResources/StandardMacros.IncrementInt` (`KismetMathLibrary.FTrunc` (`self.TotalSoulsSpawned`)))
    (:`  `
      (set `self.TotalSoulsSpawned` (`KismetMathLibrary.Conv_IntToDouble` _result)))))

(event `CreateSoulFloatingSpline`
  (bind (_returnvalue_x _returnvalue_y _returnvalue_z) (`KismetMathLibrary.BreakVector` (`self.K2_GetActorLocation` (`self.Player`))))
  (bind _returnvalue (`|SpawnActorFromClass` "/Game/GameJam2023/Blueprints/General/Soul/BP_SoulFloating.BP_SoulFloating_C" (`self.GetTransform` (`self.Player`)) "Undefined" "OverrideRootScale" null (`self.CaughtSouls`) null))
  (`self.K2_AttachToActor` _returnvalue (`self.Player`) "head" "SnapToTarget" "KeepRelative" "KeepRelative" true)
  (`self.K2_SetActorLocation` _returnvalue (`KismetMathLibrary.MakeVector` _returnvalue_x _returnvalue_y (+ _returnvalue_z 130.0)) false false))

(event `VerificaQuest`
  (switch `string` (`/Game/ThirdPersonBP/Blueprints/ThirdPersonCharacter.CurrentObjective` (`self.Player`))
    (:`villano`
      (`KismetSystemLibrary.PrintString` "Funciona...!"))))

(fn `Set Percentage Score`
  (params (SoulCounter :type "Float (double-precision)") (TotalSoulSpawned :type "Float (double-precision)"))
  (returns (FinalPercentaje :type "Float (double-precision)"))
  (return (* 100 (/ SoulCounter TotalSoulSpawned))))

(fn `UserConstructionScript`)