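; BP_WaterDeathZone is a water kill volume that plays a drowning sequence and respawns the player at a RespawnPoint.
; Overlapping DeathCollision with a valid RespawnPoint tilts the character relative to the follow camera, plays a swimming montage, disables input and shows WBP_WaterDeath.
; After a delay it moves the character to the RespawnPoint and resets rotation, then shortly clears all widgets and restores input.
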(event `self.DeathCollision.OnComponentBeginOverlap`
  (params (OverlappedComponent :type "PrimitiveComponent Object Reference") (OtherActor :type "Actor Object Reference") (OtherComp :type "PrimitiveComponent Object Reference") (OtherBodyIndex :type Integer) (bFromSweep :type Boolean) (SweepResult :type "HitResult Structure (by ref)"))
  (bind _asthird_person_character (cast `/Game/ThirdPersonBP/Blueprints/ThirdPersonCharacter` OtherActor))
  (set `self.Player` _asthird_person_character)
  (`/Engine/EditorBlueprintResources/StandardMacros.IsValid` (`self.RespawnPoint`)
    (:`Is Valid`
      (`self.PlayerStartDrowning`)
      (`KismetSystemLibrary.Delay` 2.5)
      (`self.PlayerEndDrowning`))))

(event `PlayerStartDrowning`
  (bind _returnvalue (`GameplayStatics.GetPlayerController` 0))
  (bind _player (`self.Player`))
  (`self.K2_SetActorRotation` (`self.Player`) (`KismetMathLibrary.MakeRotator` (.roll (`KismetMathLibrary.FindLookAtRotation` (`self.K2_GetActorLocation` _player) (`SceneComponent.K2_GetComponentLocation` (`/Game/ThirdPersonBP/Blueprints/ThirdPersonCharacter.FollowCamera` _player)))) (+ (.pitch (`KismetMathLibrary.FindLookAtRotation` (`self.K2_GetActorLocation` _player) (`SceneComponent.K2_GetComponentLocation` (`/Game/ThirdPersonBP/Blueprints/ThirdPersonCharacter.FollowCamera` _player)))) 90.0) (.yaw (`KismetMathLibrary.FindLookAtRotation` (`self.K2_GetActorLocation` _player) (`SceneComponent.K2_GetComponentLocation` (`/Game/ThirdPersonBP/Blueprints/ThirdPersonCharacter.FollowCamera` _player))))) false)
  (`Character.PlayAnimMontage` (`self.Player`) "/Game/GameJam2023/Animations/Player/Animation/Swimming_Montage.Swimming_Montage" 2.0 "None")
  (`self.DisableInput` (`self.Player`) _returnvalue)
  (bind _returnvalue_2 (`|CreateWidget` "/Game/GameJam2023/UI/WaterDeath/WBP_WaterDeath.WBP_WaterDeath_C" _returnvalue))
  (set `self.WBP_WaterDeath` _returnvalue_2)
  (`UserWidget.AddToViewport` _returnvalue_2 0))

(event `PlayerEndDrowning`
  (`self.K2_SetActorLocation` (`self.Player`) (`self.K2_GetActorLocation` (`self.RespawnPoint`)) false false)
  (`Character.StopAnimMontage` (`self.Player`) "/Game/GameJam2023/Animations/Player/Animation/Swimming_Montage.Swimming_Montage")
  (`self.K2_SetActorRotation` :`self` (`self.Player`))
  (`KismetSystemLibrary.Delay` 0.6)
  (`WidgetLayoutLibrary.RemoveAllWidgets`)
  (`self.EnableInput` (`self.Player`) (`GameplayStatics.GetPlayerController` 0)))

(fn `UserConstructionScript`)