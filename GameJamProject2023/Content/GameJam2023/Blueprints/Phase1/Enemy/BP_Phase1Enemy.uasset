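; Phase 1 enemy pawn that spins in place to scan and moves toward the player character when it sees them.
; PawnSensing sightings pause RotatingMovement, send a simple move to the player's current location, and start a one-second timer that resumes the spin.
; Ground friction and walking braking are zeroed at BeginPlay, so the enemy slides with momentum.
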(event `self.ReceiveBeginPlay`
  (bind _charactermovement (`self.CharacterMovement`))
  (set `RotatingMovementComponent.RotationRate` (`KismetMathLibrary.MakeRotator` 0.0 0.0 (`self.ZRotation`)) (`self.RotatingMovement`))
  (set `CharacterMovementComponent.GroundFriction` 0.0 _charactermovement)
  (set `CharacterMovementComponent.BrakingDecelerationWalking` 0.0 _charactermovement))

(event `self.PawnSensing.OnSeePawn`
  (params (Pawn :type "Pawn Object Reference"))
  (bind _asthird_person_character (cast `/Game/ThirdPersonBP/Blueprints/ThirdPersonCharacter` Pawn)
    (:`then`
      (`ActorComponent.Deactivate` (`self.RotatingMovement`))
      (`AIBlueprintHelperLibrary.SimpleMoveToLocation` (`self.GetController` self) (`self.K2_GetActorLocation` _asthird_person_character))
      (bind _returnvalue (`KismetSystemLibrary.K2_SetTimerDelegate` (delegate `ActivateRotating`) 1.0)))
    (:`CastFailed`
      (`KismetSystemLibrary.PrintString` "Cant see youuu!" true false (struct :`R` 1.0 :`B` 0.113624 :`A` 1.0) 0.5))))

(event `ActivateRotating`
  (`ActorComponent.SetActive` (`self.RotatingMovement`) true false)
  (`KismetSystemLibrary.K2_ClearAndInvalidateTimerHandle` (stale `self.PawnSensing.OnSeePawn` _returnvalue)))

(fn `UserConstructionScript`)