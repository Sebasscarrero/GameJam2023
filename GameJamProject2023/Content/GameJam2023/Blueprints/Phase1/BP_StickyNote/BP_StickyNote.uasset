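; BP_StickyNote is a sticky note actor that shows a text label on a randomly colored plane.
; On BeginPlay it copies its Text variable into the TextRender component.
; It then creates a dynamic instance of M_StickyNote on the Plane and sets the NoteColor parameter to random RGB values, so the color is picked at runtime.
; The construction script is empty.
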(event `self.ReceiveBeginPlay`
  (`TextRenderComponent.K2_SetText` (`self.TextRender`) (`self.Text`))
  (bind _returnvalue (`PrimitiveComponent.CreateDynamicMaterialInstance` (`self.Plane`) 0 "/Game/GameJam2023/Blueprints/Phase1/BP_StickyNote/M_StickyNote.M_StickyNote" "None"))
  (`PrimitiveComponent.SetMaterial` (`self.Plane`) 0 _returnvalue)
  (`MaterialInstanceDynamic.SetVectorParameterValue` _returnvalue "NoteColor" (make `LinearColor` (`KismetMathLibrary.RandomFloat`) (`KismetMathLibrary.RandomFloat`) (`KismetMathLibrary.RandomFloat`) 1.0)))

(fn `UserConstructionScript`)