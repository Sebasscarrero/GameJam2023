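; Statue actor for Phase 3 that stages a talk-to-statue moment when the ThirdPersonCharacter enters its box collision.
; On overlap it starts moving the character toward a PlayerPosition goal and caches a look-at rotation from their current location to the statue body.
; After a short delay, a timeline lerps the character to that rotation while the talking montage plays and input is disabled, with no re-enable here.
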(event `self.BoxCollision.OnComponentBeginOverlap`
  (params (OverlappedComponent :type "PrimitiveComponent Object Reference") (OtherActor :type "Actor Object Reference") (OtherComp :type "PrimitiveComponent Object Reference") (OtherBodyIndex :type Integer) (bFromSweep :type Boolean) (SweepResult :type "HitResult Structure (by ref)"))
  (bind _character (`self.Character`))
  (bind _asthird_person_character (cast `/Game/ThirdPersonBP/Blueprints/ThirdPersonCharacter` OtherActor))
  (set `self.Character` _asthird_person_character)
  (`AIBlueprintHelperLibrary.SimpleMoveToActor` (`Pawn.GetController` _asthird_person_character) (`self.PlayerPosition`))
  (set `self.RotationToStatue` (`KismetMathLibrary.FindLookAtRotation` (`self.K2_GetActorLocation` (`self.Character`)) (`SceneComponent.K2_GetComponentLocation` (`self.StatueBody`))))
  (`KismetSystemLibrary.Delay` 0.5)
  (`|ExecutionSequence`
    (:`then_0`
      (bind (_direction _speed) (`Timeline|RotatePlayerToStatue` :!via `PlayFromStart`)
        (:`Update`
          (`self.K2_SetActorRotation` _character (`KismetMathLibrary.RLerp` (`self.K2_GetActorRotation` _character) (`self.RotationToStatue`) _speed) false))))
    (:`then_1`
      (`Character.PlayAnimMontage` (`self.Character`) "/Game/GameJam2023/Animations/Player/Character_Talking_Statue_Montage.Character_Talking_Statue_Montage" 1.0 "None")
      (`self.DisableInput` (`self.Character`) (`GameplayStatics.GetPlayerController` 0)))))

(fn `UserConstructionScript`)